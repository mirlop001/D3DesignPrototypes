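; BP_Hook is a grappling hook that pulls its owning Character toward whatever the hook hits.
; LaunchHook spawns a BP_GrappleHook projectile with an attached cable and binds its hit and destroy events.
; On hit, it removes gravity and ground friction and sets velocity toward the hook, then Tick keeps adding force.
; The hook is destroyed on proximity, overshoot or cancel, which clears the cable and resets movement settings.
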(event `self.ReceiveTick`
  (params (DeltaSeconds :type "Float (single-precision)"))
  (switch `/Game/Blueprints/Hook/BP_HookState` (`self.HookState`)
    (:`NewEnumerator2`
      (bind _ascharacter (cast `Character` (`self.GetOwner`)))
      (`CharacterMovementComponent.AddForce` (`Character.CharacterMovement` _ascharacter) (* (`self.ToHook`) 100000.0))
      (if (< (`KismetMathLibrary.Vector_Distance` (`Actor.K2_GetActorLocation` (`self.GrappleHook`)) (`Actor.K2_GetActorLocation` (`self.GetOwner`))) 250.0)
        (`Actor.K2_DestroyActor` (`self.GrappleHook`))
        (elif (< (`KismetMathLibrary.Dot_VectorVector` (`self.InitialHookDirection2D`) (`self.ToGrappleHook2D`)) 0.0)
          (`Actor.K2_DestroyActor` (`self.GrappleHook`)))))))

(fn `CancelLaunchHook`
  (bind _grapplehook (`self.GrappleHook`)
    (:`then`
      (`Actor.K2_DestroyActor` _grapplehook))
    (:`else`)))

(fn `IsInUse`
  (returns (Result :type Boolean))
  (return (select `/Game/Blueprints/Hook/BP_HookState` (`self.HookState`) :`NewEnumerator1` true :`NewEnumerator2` true)))

(fn `LaunchHook`
  (params (TargetLocation :type "Vector Structure") (LocalOffset :type "Vector Structure"))
  (locals (FireDirection :type "Vector Structure"))
  (bind _result (`self.IsInUse`))
  (if (not _result)
    (set `local.FireDirection` (`KismetMathLibrary.Normal` (- (`local.TargetLocation`) (`self.StartHookLocation` (`local.LocalOffset`)))))
    (bind _returnvalue (`|SpawnActorFromClass` "/Game/Blueprints/Hook/BP_GrappleHook.BP_GrappleHook_C" (`KismetMathLibrary.MakeTransform` (`self.StartHookLocation` (`local.LocalOffset`))) "Undefined" "OverrideRootScale" null (* (`local.FireDirection`) (`self.Speed`)) null))
    (bind _output_get (set `self.GrappleHook` _returnvalue))
    (add `Actor.OnActorHit` _output_get (`|CreateDelegate` :!event `OnGrappleHit`))
    (add `Actor.OnDestroyed` (`self.GrappleHook`) (`|CreateDelegate` :!event `OnGrappleDestroy`))
    (bind _returnvalue_2 (`|SpawnActorFromClass` "/Game/Blueprints/Hook/BP_HookCable.BP_HookCable_C" (`KismetMathLibrary.MakeTransform` (`self.StartHookLocation` (`local.LocalOffset`)) (`KismetMathLibrary.MakeRotFromX` (`local.FireDirection`))) "Undefined" "OverrideRootScale" null null))
    (bind _output_get_2 (set `self.GrappleCable` _returnvalue_2))
    (`Actor.K2_AttachToActor` _output_get_2 (`self.GetOwner`) "None" "KeepWorld" "KeepWorld" "KeepWorld" true)
    (`CableComponent.SetAttachEndTo` (`CableActor.CableComponent` (`self.GrappleCable`)) (`self.GrappleHook`) "None" "None")
    (set `CableComponent.EndLocation` (0.0 0.0 0.0) (`CableActor.CableComponent` (`self.GrappleCable`)))
    (return)))

(fn `OnGrappleDestroy`
  (params (DestroyedActor :type "Actor Object Reference"))
  (bind _grapplehook (`self.GrappleHook`)
    (:`then`
      (`Actor.K2_DestroyActor` _grapplehook)
      (set `self.GrappleHook` null)
      (set `self.HookState` "NewEnumerator0")
      (`|ExecutionSequence`
        (:`then_0`
          (bind _grapplecable (`self.GrappleCable`)
            (:`then`
              (`Actor.K2_DestroyActor` _grapplecable)
              (set `self.GrappleCable` null))
            (:`else`)))
        (:`then_1`
          (bind _ascharacter (cast `Character` (`self.GetOwner`)))
          (bind _charactermovement (`Character.CharacterMovement` _ascharacter))
          (set `CharacterMovementComponent.GroundFriction` 1.0 _charactermovement)
          (set `CharacterMovementComponent.GravityScale` 1.0 _charactermovement)
          (set `CharacterMovementComponent.AirControl` 0.05 _charactermovement))))
    (:`else`)))

(fn `OnGrappleHit`
  (params (SelfActor :type "Actor Object Reference") (OtherActor :type "Actor Object Reference") (NormalImpulse :type "Vector Structure") (Hit :type "HitResult Structure (by ref)"))
  (set `self.HookState` "NewEnumerator2")
  (bind _ascharacter (cast `Character` (`self.GetOwner`)))
  (bind _charactermovement (`Character.CharacterMovement` _ascharacter))
  (set `CharacterMovementComponent.GroundFriction` 0.0 _charactermovement)
  (set `CharacterMovementComponent.GravityScale` 0.0 _charactermovement)
  (set `CharacterMovementComponent.AirControl` 0.2 _charactermovement)
  (set `MovementComponent.Velocity` (* (`self.ToHook`) 1200.0) _charactermovement)
  (set `self.InitialHookDirection2D` (`self.InitialHookDirection2D`))
  (return))